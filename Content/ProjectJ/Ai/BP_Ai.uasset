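; BP_Ai is an AI-controlled enemy character that attacks BP_Character and tracks its own HP.
; Once possessed by BP_AiController, a fast looping timer polls the blackboard AiState; in Attack it plays a random DT_Attack montage and immediately line-traces forward to apply damage.
; A busy flag blocks overlapping attacks and takes the montage's Interrupted value on end, so only uninterrupted endings clear it.
; Damage taken lowers clamped HP and updates an AJ_PlayerWidget.
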(event `self.ReceivePossessed`
  (params (NewController :type "Controller Object Reference"))
  ;[1 1 1] Random Attack Anim
  (if (== (`GameplayStatics.GetObjectClass` NewController) "/Game/ProjectJ/Ai/BP_AiController.BP_AiController_C")
    (`KismetSystemLibrary.K2_SetTimer` null "Ai Attack" 0.01 true)
    (add `AnimInstance.OnMontageEnded` (`SkeletalMeshComponent.GetAnimInstance` (`self.Mesh`)) (`|CreateDelegate` :!event `EventMontageEnd`))))

(event `self.ReceiveBeginPlay`
  (bind _returnvalue (`|CreateWidget` "/Game/ProjectJ/Widget/Player/AJ_PlayerWidget.AJ_PlayerWidget_C" (`GameplayStatics.GetPlayerController` 0)))
  (set `self.AjWidget` _returnvalue)
  (bind _output_get (set `self.CurHp` (`self.MaxHp`)))
  (`/Game/ProjectJ/Widget/Player/AJ_PlayerWidget.Set Hp` (`self.AjWidget`) _output_get (`self.MaxHp`) 0))

(event `self.ReceiveAnyDamage`
  (params (Damage :type "Float (single-precision)") (DamageType :type "DamageType Object Reference") (InstigatedBy :type "Controller Object Reference") (DamageCauser :type "Actor Object Reference"))
  (bind _output_get (set `self.CurHp` (`KismetMathLibrary.FClamp` (- (`self.CurHp`) Damage) 0.0 (`self.MaxHp`))))
  (`/Game/ProjectJ/Widget/Player/AJ_PlayerWidget.Set Hp` (`self.AjWidget`) _output_get (`self.MaxHp`) 0))

(fn `Ai Attack`
  (bind _returnvalue (`self.K2_GetActorLocation`))
  (bind _output_get (set `self.AiState` (cast `/Game/ProjectJ/Ai/EN_Ai` (`BlackboardComponent.GetValueAsEnum` (`AIBlueprintHelperLibrary.GetBlackboard` (`self.GetController`)) "AiState"))))
  (switch `/Game/ProjectJ/Ai/EN_Ai` _output_get
    (:`NewEnumerator2`
      (if (not (`self.IsAnimmontage`))
        (set `self.IsAnimmontage` true)
        (bind _outrownames (`DataTableFunctionLibrary.GetDataTableRowNames` "/Game/ProjectJ/Ai/DT_Attack.DT_Attack"))
        (bind _returnvalue_2 (`|GetDataTableRow` "/Game/ProjectJ/Ai/DT_Attack.DT_Attack" (`KismetArrayLibrary.Array_Random` _outrownames))
          (:`then`
            (`self.PlayAnimMontage` (`.Montage_3_28F2B1F44FB29FBABE82CAA9FDC97EB7` (break `/Game/ProjectJ/Ai/ST_Attack` _returnvalue_2)))
            (bind (_outhit _returnvalue_3) (`KismetSystemLibrary.LineTraceSingle` :`Start` _returnvalue :`End` (+ _returnvalue (* (`KismetMathLibrary.GetForwardVector` (`self.K2_GetActorRotation`)) 200.0)) :`TraceChannel` "TraceTypeQuery1" :`DrawDebugType` "ForDuration"))
            (if _returnvalue_3
              (bind _asbp_character (cast `/Game/ProjectJ/Blueprints/BP_Character` (`.HitActor` (`GameplayStatics.BreakHitResult` _outhit))))
              (`GameplayStatics.ApplyDamage` _asbp_character (`self.Base Damage`) (`self.GetController`) self)
              (`KismetSystemLibrary.PrintString` "해냈다해냈어")
              (else
                (`KismetSystemLibrary.PrintString` "AttackFalse")))))))))

(fn `EventMontageEnd`
  (params (Montage :type "AnimMontage Object Reference") (bInterrupted :type Boolean))
  (set `self.IsAnimmontage` bInterrupted))

(fn `UserConstructionScript`)