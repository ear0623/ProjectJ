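; BP_PlayerHUD is the player HUD Blueprint that relays the player's health, STM, ammo and magazine values to the on-screen widget.
; Each OnUpdateMy event casts HudWidget to AJ_PlayerWidget and calls the matching setter, stopping if the cast fails.
; BeginPlay caches the cast widget, but the update events cast again instead of using that reference.
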(event `self.ReceiveBeginPlay`
  (bind _asaj_player_widget (cast `/Game/ProjectJ/Widget/Player/AJ_PlayerWidget` (`self.HudWidget`)))
  (set `self.As AJ Player Widget` _asaj_player_widget))

(event `self.OnUpdateMyHp`
  (params (CurHp :type "Float (single-precision)") (MaxHp :type "Float (single-precision)") (CurHpText :type Integer))
  (bind _asaj_player_widget (cast `/Game/ProjectJ/Widget/Player/AJ_PlayerWidget` (`self.HudWidget`)))
  (`/Game/ProjectJ/Widget/Player/AJ_PlayerWidget.Set Hp` _asaj_player_widget CurHp MaxHp 0))

(event `self.OnUpdateMySTM`
  (params (CurSTM :type "Float (single-precision)") (MaxSTM :type "Float (single-precision)"))
  (bind _asaj_player_widget (cast `/Game/ProjectJ/Widget/Player/AJ_PlayerWidget` (`self.HudWidget`)))
  (`/Game/ProjectJ/Widget/Player/AJ_PlayerWidget.SetSMT` _asaj_player_widget CurSTM MaxSTM))

(event `self.OnUpdateMyAmmo`
  (params (Ammo :type Integer))
  (bind _asaj_player_widget (cast `/Game/ProjectJ/Widget/Player/AJ_PlayerWidget` (`self.HudWidget`)))
  (`/Game/ProjectJ/Widget/Player/AJ_PlayerWidget.SetAmmo` _asaj_player_widget Ammo))

(event `self.OnUpdateMyMag`
  (params (Mag :type Integer))
  (bind _asaj_player_widget (cast `/Game/ProjectJ/Widget/Player/AJ_PlayerWidget` (`self.HudWidget`)))
  (`/Game/ProjectJ/Widget/Player/AJ_PlayerWidget.SetMag` _asaj_player_widget Mag))

(fn `UserConstructionScript`)