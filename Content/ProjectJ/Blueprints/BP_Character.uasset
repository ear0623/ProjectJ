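; BP_Character is a character Blueprint with health, a short-range attack and death.
; BeginPlay caches the player HUD and fills health; AnyDamage clamps health, updates the HUD's AJ_PlayerWidget and calls Death at zero.
; Left mouse press line-traces a short distance forward and applies fixed damage to any AJ_Character hit.
; Death plays a death montage, disables capsule collision and turns on mesh physics simulation for a ragdoll.
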(event `self.ReceiveBeginPlay`
  (bind _asbp_player_hud (cast `/Game/ProjectJ/Blueprints/Player/BP_PlayerHUD` (`PlayerController.GetHUD` (`GameplayStatics.GetPlayerController` 0))))
  (set `self.As BP Player HUD` _asbp_player_hud)
  (set `self.CurHp` (`self.MaxHp`)))

(event `self.ReceiveAnyDamage`
  (params (Damage :type "Float (single-precision)") (DamageType :type "DamageType Object Reference") (InstigatedBy :type "Controller Object Reference") (DamageCauser :type "Actor Object Reference"))
  (bind _output_get (set `self.CurHp` (`KismetMathLibrary.FClamp` (- (`self.CurHp`) Damage) 0.0 (`self.MaxHp`))))
  (bind _asaj_player_widget (cast `/Game/ProjectJ/Widget/Player/AJ_PlayerWidget` (`PlayerHUD.HudWidget` (`self.As BP Player HUD`))))
  (`/Game/ProjectJ/Widget/Player/AJ_PlayerWidget.Set Hp` _asaj_player_widget _output_get (`self.MaxHp`) 0)
  (if (== (`self.CurHp`) 0.0)
    (`self.death`)))

(event `Key|LeftMouseButton`
  (params (Key :type "Key Structure"))
  (bind _returnvalue (`self.K2_GetActorLocation`))
  (:`Pressed`
    (bind (_outhit _returnvalue_2) (`KismetSystemLibrary.LineTraceSingle` _returnvalue (+ _returnvalue (* (`KismetMathLibrary.GetForwardVector` (`self.K2_GetActorRotation`)) 200.0)) "TraceTypeQuery1"))
    (if _returnvalue_2
      (bind _asaj_character (cast `AJ_Character` (`.HitActor` (`GameplayStatics.BreakHitResult` _outhit))))
      (`GameplayStatics.ApplyDamage` _asaj_character 34.0 (`self.GetController`) self))))

(fn `death`
  (`SkeletalMeshComponent.PlayAnimation` (`self.Mesh`) "/Game/Characters/Mannequins/Animations/InPlace/Rifle_Death_R_Montage.Rifle_Death_R_Montage" false)
  (`PrimitiveComponent.SetCollisionEnabled` (`self.CapsuleComponent`) "NoCollision")
  (`PrimitiveComponent.SetSimulatePhysics` (`self.Mesh`) true))

(fn `UserConstructionScript`)